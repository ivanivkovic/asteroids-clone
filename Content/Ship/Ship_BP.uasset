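; Player ship Blueprint that tracks lives and score and removes the intro HUD on the first shot.
; Each hit costs a life, then destroys the ship and spawns a fresh copy at a fixed point, carrying Lives and Score over.
; Running out swaps the HUD for Game Over, hides the ship, reassigns the controller ID and quits after a delay.
; A separate TakeDamage function decrements lives with clamping, unused by the hit logic.
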(event `self.Ship1.OnFirstShot`
  ;[1 1 1] Remove intro HUD
  (bind _foundwidgets (`WidgetBlueprintLibrary.GetAllWidgetsOfClass` "/Game/UI/IntroHUD_BP.IntroHUD_BP_C" false))
  (`Widget.RemoveFromParent` _foundwidgets))

(event `self.ReceiveHit`
  (params (MyComp :type "PrimitiveComponent Object Reference") (Other :type "Actor Object Reference") (OtherComp :type "PrimitiveComponent Object Reference") (bSelfMoved :type Boolean) (HitLocation :type "Vector Structure") (HitNormal :type "Vector Structure") (NormalImpulse :type "Vector Structure") (Hit :type "HitResult Structure (by ref)"))
  (bind _lives (`self.Lives`))
  ;[1 1 1] Ship On Hit
  (`KismetSystemLibrary.PrintString` (`KismetStringLibrary.Concat_StrStr` "Ship destroyed at " (`KismetStringLibrary.Conv_VectorToString` (`self.K2_GetActorLocation`))) false)
  (set `self.Lives` (- _lives 1))
  (if (< _lives 0)
    ;[1 1 1] No lives, Game Over
    (bind _foundwidgets (`WidgetBlueprintLibrary.GetAllWidgetsOfClass` "/Game/UI/HUD.HUD_C"))
    (`Widget.RemoveFromParent` _foundwidgets)
    (bind _returnvalue (`|CreateWidget` "/Game/UI/GameOver_BP.GameOver_BP_C"))
    (`UserWidget.AddToViewport` _returnvalue 0)
    (`SceneComponent.SetVisibility` (`self.Ship`) false false)
    (`GameplayStatics.SetPlayerControllerID` (`GameplayStatics.GetPlayerController` 0) 10)
    (`KismetSystemLibrary.Delay` 3.0)
    (`KismetSystemLibrary.QuitGame` null "Quit" true)
    (else
      ;[1 1 1] Lose life, respawn
      (`self.K2_DestroyActor`)
      (bind _returnvalue_2 (`|SpawnActorFromClass` "Ship_BP_C" (`KismetMathLibrary.MakeTransform` (0.0 0.0 200.0) (struct :`Yaw` 270.0)) "Undefined" "OverrideRootScale" null null))
      (set `/Game/Ship/Ship_BP.Lives` (`self.Lives`) _returnvalue_2)
      (set `/Game/Ship/Ship_BP.Score` (`self.Score`) _returnvalue_2))))

(fn `TakeDamage`
  (set `self.Lives` (`KismetMathLibrary.Clamp` (- (`self.Lives`) 1) 0 (`self.Max Lives`))))

(fn `UserConstructionScript`)